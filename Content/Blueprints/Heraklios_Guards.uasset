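; Heraklios guard character that carries a staff, performs a melee attack animation and dies when its health runs out.
; On BeginPlay it spawns a scaled-down Wooden_Staff and snaps it to the Weapon socket of a child component.
; Attack plays a sword slash, gated by a DoOnce that resets after a short delay.
; Damage reduces Health; at zero it spawns an explosion, calls GuardDeath and destroys both staff and guard.
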(event Custom|Attack
  (Utilities|FlowControl|DoOnce false :!label _label
    (:Completed
      (Components|Animation|PlayAnimation "/Game/MixamoAnimPack/Mixamo_Heraklios/Anims/Mixamo_Heraklios_Sword_Slash.Mixamo_Heraklios_Sword_Slash" false)
      (Utilities|FlowControl|Delay 1.5)
      (goto _label Reset))))

(event EventAnyDamage
  (params (Damage :type Float%20%28single-precision%29) (DamageType :type Damage%20Type%20Object%20Reference) (InstigatedBy :type Controller%20Object%20Reference) (DamageCauser :type Actor%20Object%20Reference))
  (Variables|Default|SetHealth (- (Variables|Default|GetHealth) Damage))
  (if (<= (Variables|Default|GetHealth) 0.0)
    (Effects|SpawnEmitteratLocation "/Game/StarterContent/Particles/P_Explosion.P_Explosion" (Transformation|GetActorLocation))
    (Default|CallGuardDeath)
    (Actor|DestroyActor (stale EventBeginPlay _returnvalue))
    (Actor|DestroyActor)))

(event EventBeginPlay
  (bind _returnvalue (Game|SpawnActorfromClass "/Game/Blueprints/Wooden_Staff.Wooden_Staff_C" (Transformation|GetActorTransform) false 0))
  (Transformation|SetActorScale3D _returnvalue "0.100000,0.100000,0.100000")
  (Class|Actor|AttachRootComponentto _returnvalue (Components|GetChildComponent (VehicleSound|GetRootComponent) 2) "Weapon" "SnapToTarget" true))

(event EventTick
  (params (DeltaSeconds :type Float%20%28single-precision%29)))

(fn ConstructionScript)