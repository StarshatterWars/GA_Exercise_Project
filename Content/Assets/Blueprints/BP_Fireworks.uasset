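; Fireworks actor that plays particle bursts with takeoff and explosion sounds, in either single-burst or multi-burst mode.
; Single-burst mode loops on a random delay, adding a new particle component each pass, optionally at a random XY offset.
; Multi-burst mode uses one component created in the Construction Script.
; Both modes bind particle spawn and death events, matching event names to play sounds, optionally at the particle's location.
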(event Custom|OnParticleDeath_Event_0_Copy
  (params (EventName :type Name :default "None") (EmitterTime :type Float%20%28single-precision%29) (ParticleTime :type Integer) (Location :type Vector :default "0, 0, 0") (Velocity :type Vector) (Direction :type Vector))
  (bind _bshoulduseexplosionlocationforaudio (Variables|Default|GetbShouldUseExplosionLocationForAudio))
  (bind _returnvalue (Math|Vector|SelectVector Location "0, 0, 0" _bshoulduseexplosionlocationforaudio))
  ;[1 1 1] Same As Above But For Multiple Burst
  (Utilities|FlowControl|Sequence
    (:then_0
      (if (Utilities|Name|Equal(Name) EventName "First")
        (Audio|PlaySoundatLocation (Variables|Default|GetMainExplosionSoundCue) _returnvalue)))
    (:then_1
      (if (Utilities|Name|Equal(Name) EventName "Second")
        (Audio|PlaySoundatLocation (Variables|Default|GetSecondaryExplosionSoundCue) _returnvalue)))))

(event Custom|OnParticleSpawn_Event_0_Copy
  (params (EventName :type Name :default "None") (EmitterTime :type Float%20%28single-precision%29) (Location :type Vector :default "0, 0, 0") (Velocity :type Vector))
  ;[1 1 1] Same As Above But For Multiple Burst
  (if (Utilities|Name|Equal(Name) EventName "LeadSpawn")
    (Audio|PlaySoundatLocation (Variables|Default|GetTakeoffSoundCue) (Math|Vector|SelectVector Location "0, 0, 0" (Variables|Default|GetbShouldUseExplosionLocationForAudio)))))

(event Custom|OnParticleDeath_Event_0
  (params (EventName :type Name :default "None") (EmitterTime :type Float%20%28single-precision%29) (ParticleTime :type Integer) (Location :type Vector :default "0, 0, 0") (Velocity :type Vector) (Direction :type Vector))
  (bind _bshoulduseexplosionlocationforaudio (Variables|Default|GetbShouldUseExplosionLocationForAudio))
  (bind _returnvalue (Math|Vector|SelectVector Location "0, 0, 0" _bshoulduseexplosionlocationforaudio))
  ;[1 1 1] Binds An Event to The Explosions (First And Secondary)
  (Utilities|FlowControl|Sequence
    (:then_0
      (if (Utilities|Name|Equal(Name) EventName "First")
        (Audio|PlaySoundatLocation (Variables|Default|GetMainExplosionSoundCue) _returnvalue)))
    (:then_1
      (if (Utilities|Name|Equal(Name) EventName "Second")
        (Audio|PlaySoundatLocation (Variables|Default|GetSecondaryExplosionSoundCue) _returnvalue)))))

(event Custom|OnParticleSpawn_Event_0
  (params (EventName :type Name :default "None") (EmitterTime :type Float%20%28single-precision%29) (Location :type Vector :default "0, 0, 0") (Velocity :type Vector))
  ;[1 1 1] Binds An Event To The initial Particle Takeoff
  (if (Utilities|Name|Equal(Name) EventName "LeadSpawn")
    (Audio|PlaySoundatLocation (Variables|Default|GetTakeoffSoundCue) (Math|Vector|SelectVector Location "0, 0, 0" (Variables|Default|GetbShouldUseExplosionLocationForAudio)))))

(event EventBeginPlay
  (bind _spawnradius (Variables|Default|GetSpawnRadius))
  ;[1 1 1] Comment
  ;;[1 1 1] Starts Spawning For Single Burst Particle
  (if (Variables|Default|GetbSingleOrMultiBurst)
    (Utilities|FlowControl|Sequence :!label _label
      (:then_0
        (Utilities|FlowControl|Delay (Math|Random|RandomFloatinRange (Variables|Default|GetMinSpawnTime) (Variables|Default|GetMaxSpawnTime)))
        (goto _label))
      (:then_1
        ;[1 1 1] Generates Particle Component
        (bind _returnvalue (AddComponent|AddParticleSystemComponent false (Math|Conversions|ToTransform(Vector) (Math|Vector|SelectVector (Math|Vector|MakeVector (* (Math|Random|RandomFloatinRange 1.0 -1.0) _spawnradius) (* (Math|Random|RandomFloatinRange 1.0 -1.0) _spawnradius) 0.0) "0, 0, 0" (and (Variables|Default|GetbSingleOrMultiBurst) (Variables|Default|GetbIfSingleBurstShouldMoveLocation))))))
        (Effects|Components|ParticleSystem|SetTemplate _returnvalue (Utilities|Array|Get(acopy) (Variables|Default|GetParticleAssetArray) (Math|Integer|SelectInt 1 0 (Variables|Default|GetbSingleOrMultiBurst))))
        ;[1 1 1] Binds An Event to The Explosions (First And Secondary)
        (EventDispatchers|AssignOnParticleDeath _returnvalue (delegate Custom|OnParticleDeath_Event_0))
        ;[1 1 1] Binds An Event To The initial Particle Takeoff
        (EventDispatchers|AssignOnParticleSpawn _returnvalue (delegate Custom|OnParticleSpawn_Event_0))))
    (else
      ;[1 1 1] Same As Above But For Multiple Burst
      (EventDispatchers|AssignOnParticleDeath (Variables|Default|GetBurstParticleComponent) (delegate Custom|OnParticleDeath_Event_0_Copy))
      ;[1 1 1] Same As Above But For Multiple Burst
      (EventDispatchers|AssignOnParticleSpawn (Variables|Default|GetBurstParticleComponent) (delegate Custom|OnParticleSpawn_Event_0_Copy)))))

(fn ConstructionScript
  (if (not (Variables|Default|GetbSingleOrMultiBurst))
    (bind _returnvalue (AddComponent|AddParticleSystemComponent false))
    (Effects|Components|ParticleSystem|SetTemplate _returnvalue (Utilities|Array|Get(acopy) (Variables|Default|GetParticleAssetArray) (Math|Integer|SelectInt 1 0 (Variables|Default|GetbSingleOrMultiBurst))))
    (Variables|Default|SetBurstParticleComponent _returnvalue)))